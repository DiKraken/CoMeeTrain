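; Game mode that holds the water and coal resources and a letter pickup state for BP_Player.
; CheckConditions restarts the level when either resource is depleted, otherwise slows or restores player speed based on the water-coal gap.
; Helpers update resource values on the widget and relay letter changes to the player and lines manager.
; BeginPlay only caches the player; widget creation, resource timer, manager lookup and speed display are disconnected.
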(event `self.ReceiveBeginPlay`
  (bind _asbp_player (cast `/Game/Base/BP_Player` (`GameplayStatics.GetPlayerPawn` 0)))
  (set `self.Player` _asbp_player))

(event `ResourceTick`)

(event `CheckConditions`
  (bind _player (`self.Player`))
  (if (not (or (<= (`self.WaterValue`) 0.0) (<= (`self.CoalValue`) 0.0)))
    (`self.WaterCoalRatioCheck`
      (:`True`
        (if (`/Game/Base/BP_Player.SpeedUp` _player)
          (`/Game/Base/BP_Player.SlowDownToNormal` _player)
          (`KismetSystemLibrary.Delay` 0.5)
          (`/Game/Base/BP_Player.Slow Down` _player)
          (else
            (`/Game/Base/BP_Player.Slow Down` _player))))
      (:`False`
        (`/Game/Base/BP_Player.SpeedUpToNormal` _player)))
    (else
      (`self.RestartLevel`))))

(event `self.ReceiveTick`
  (params (DeltaSeconds :type "Float (single-precision)")))

(fn `AddCoal`
  (params (Value :type "Float (double-precision)"))
  (bind _output_get (set `self.CoalValue` (+ Value (`self.CoalValue`))))
  (bind _widget (`self.Widget`)
    (:`then`
      (`/Game/UI/W_UI.SetCoal` _widget _output_get))
    (:`else`)))

(fn `AddLetter`
  (set `self.Letter?` true)
  (`/Game/Base/BP_Player.AddLetter` (`self.Player`)))

(fn `AddWater`
  (params (Value :type "Float (double-precision)"))
  (bind _output_get (set `self.WaterValue` (+ Value (`self.WaterValue`))))
  (`self.Widget`
    (:`then`
      (`/Game/UI/W_UI.SetWater` (`self.Widget`) _output_get))
    (:`else`)))

(fn `RemoveLetter`
  (set `self.Letter?` false)
  (`/Game/Base/BP_Player.RemoveLetter` (`self.Player`))
  (`/Game/Blueprints/BP_LinesManager.IncreaseEachNSeg` (`self.LinesManager`) 2.0))

(fn `RestartLevel`
  (bind _returnvalue (`GameplayStatics.GetCurrentLevelName` true))
  (`GameplayStatics.OpenLevel` (`KismetStringLibrary.Conv_StringToName` _returnvalue)))

(fn `SetTickValue`
  (params (TickValue :type "Float (double-precision)"))
  (set `self.TickValue` TickValue))

(fn `UserConstructionScript`)