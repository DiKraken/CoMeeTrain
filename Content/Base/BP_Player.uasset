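; BP_Player is an auto-forward runner player that sidesteps between lanes and restarts the level when it falls.
; Tick drives swept forward movement at a speed the Slow timeline blends between normal and slow.
; Left/right inputs play timelines shifting one fixed lane step within borders set by SetBorders.
; CheckUnder traces down after a delay; without ground, it stops movement, breaks constraints, launches physics pieces, then reloads the level.
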(event `Slow Down`
  (set `self.SlowDown` true)
  (bind (_direction _value) (`Timeline|Slow` :!label _label)
    (:`Update`
      (set `self.MovementSpeed` (`KismetMathLibrary.Lerp` (`self.NormalMovementSpeed`) (`self.SlowMovementSpeed`) _value)))))

(event `self.ReceiveTick`
  (params (DeltaSeconds :type "Float (single-precision)"))
  ;[0.1593 1 0.06256] PlayerMovement
  ;;[1 1 1] ForwardMovement
  (`self.K2_AddActorLocalOffset` (`KismetMathLibrary.MakeVector` (* DeltaSeconds (`self.MovementSpeed`))) true))

(event `SpeedUpToNormal`
  (if (`self.SlowDown`)
    (set `self.SlowDown` false)
    (goto _label :!via `Reverse`)))

(event `InputAction|MoveRight`
  (params (Key :type "Key Structure"))
  (bind (_returnvalue_x _returnvalue_y) (`KismetMathLibrary.BreakVector` (`self.K2_GetActorLocation`)))
  (bind (_returnvalue_x_2 _returnvalue_y_2 _returnvalue_z) (`KismetMathLibrary.BreakVector` (`self.K2_GetActorLocation`)))
  (bind (_initlocation_x _initlocation_y) (`KismetMathLibrary.BreakVector` (`self.InitLocation`)))
  ;[0.1593 1 0.06256] PlayerMovement
  ;;[1 1 1] RightLeftMovement
  (:`Pressed`
    (if (not (or (>= _returnvalue_y (`self.MovementBorderRight`)) (`self.MovingRL`)))
      (set `self.MovingRL` true)
      (set `self.InitLocation` (`self.K2_GetActorLocation`))
      (bind (_direction _value) (`Timeline|MoveRight` :!via `PlayFromStart` :!label _label_2)
        (:`Update`
          (`self.K2_SetActorRelativeLocation` (`KismetMathLibrary.MakeVector` _returnvalue_x_2 (`KismetMathLibrary.Lerp` _initlocation_y (+ _initlocation_y 150.0) _value) _returnvalue_z) true))
        (:`Finished`
          (set `self.MovingRL` false :!label _label_3))))))

(event `StopMovement`
  (bind (_returnvalue_x _returnvalue_y _returnvalue_z) (`KismetMathLibrary.BreakVector` (`self.K2_GetActorLocation`)))
  (bind (_initlocation_x _initlocation_y) (`KismetMathLibrary.BreakVector` (`self.InitLocation`)))
  ;[0.1593 1 0.06256] PlayerMovement
  ;;[1 1 1] RightLeftMovement
  ;;;[1 0 0] Stopper
  (`|ExecutionSequence`
    (:`then_0`
      (goto _label_2 :!via `Stop`))
    (:`then_1`
      (bind (_direction _value) (`Timeline|MoveLeft` :!via `Stop` :!label _label_4)
        (:`Update`
          (`self.K2_SetActorRelativeLocation` (`KismetMathLibrary.MakeVector` _returnvalue_x (`KismetMathLibrary.Lerp` _initlocation_y (- _initlocation_y 150.0) _value) _returnvalue_z) true))
        (:`Finished`
          (goto _label_3))))))

(event `InputAction|MoveLeft`
  (params (Key :type "Key Structure"))
  (bind (_returnvalue_x _returnvalue_y) (`KismetMathLibrary.BreakVector` (`self.K2_GetActorLocation`)))
  ;[0.1593 1 0.06256] PlayerMovement
  ;;[1 1 1] RightLeftMovement
  (:`Pressed`
    (if (not (or (`self.MovingRL`) (<= (`KismetMathLibrary.GridSnap_Float` _returnvalue_y 150.0) (`self.MovementBorderLeft`))))
      (set `self.MovingRL` true)
      (set `self.InitLocation` (`self.K2_GetActorLocation`))
      (goto _label_4 :!via `PlayFromStart`))))

(event `CheckUnder`
  ;[0.8767 0.0137 0.0137] CheckUnder
  (`KismetSystemLibrary.Delay` 0.75)
  (bind (_outhit _returnvalue) (`KismetSystemLibrary.LineTraceSingle` :`Start` (`self.K2_GetActorLocation`) :`End` (+ (`self.K2_GetActorLocation`) (0.0 0.0 -100.0)) :`TraceChannel` "TraceTypeQuery1" :`DrawTime` 1.0))
  (if (not _returnvalue)
    (`self.StopMovement`)
    (`self.SetActorTickEnabled` false)
    (`PrimitiveComponent.SetSimulatePhysics` (`self.Body`) true)
    (`PhysicsConstraintComponent.BreakConstraint` (`self.1`))
    (`PrimitiveComponent.SetEnableGravity` (`self.Cube`) true)
    (`PhysicsConstraintComponent.BreakConstraint` (`self.2`))
    (`PrimitiveComponent.SetEnableGravity` (`self.Cube1`) true)
    (`PrimitiveComponent.AddImpulse` (`self.Body`) (* (`KismetMathLibrary.RandomUnitVector`) 500.0) "None" true)
    (`self.DisableInput` null)
    (`KismetSystemLibrary.Delay` 2.0)
    (bind _returnvalue_2 (`GameplayStatics.GetCurrentLevelName` true))
    (`GameplayStatics.OpenLevel` (`KismetStringLibrary.Conv_StringToName` _returnvalue_2))))

(fn `SetBorders`
  (params (BorderLeft :type "Float (double-precision)") (BorderRight :type "Float (double-precision)"))
  (set `self.MovementBorderLeft` BorderLeft)
  (set `self.MovementBorderRight` BorderRight))

(fn `UserConstructionScript`
  (`BoxComponent.SetBoxExtent` (`self.Box`) (`.BoxExtent` (`KismetSystemLibrary.GetComponentBounds` (`self.Body`))) true))