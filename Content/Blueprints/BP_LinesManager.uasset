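; Manager for an endless road that spawns BP_RoadSegment actors along X with random line counts and left bias.
; BeginPlay pre-builds segments out to DrawDistance; SpawnSegmentSignal then adds one that far ahead of the supplied location.
; Optional cleanup is deferred a step, destroying the previously retired segment before queuing the oldest.
; Every EachNSegments signals, a FlipFlop alternately marks a letter start or end, with the interval adjustable through IncreaseEachNSeg.
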(event `self.ReceiveBeginPlay`
  (`self.SpawnSegment` (`KismetMathLibrary.MakeTransform` (1610.0 0.0 0.0)) 3)
  (for _index (range 2 (+ (`self.DrawDistance`) 1))
    (`self.SpawnSegment` (`KismetMathLibrary.MakeTransform` (* (1610.0 0.0 0.0) _index)) (`KismetMathLibrary.RandomIntegerInRange` 1 5) (`KismetMathLibrary.RandomBool`))))

(event `SpawnSegmentSignal`
  (params (`Spawn Transform Location` :type "Vector Structure") (`DeleteOld?` :type Boolean :default true))
  (if (== (mod (`self.Counter`) (`self.EachNSegments`)) 0.0)
    (`/Engine/EditorBlueprintResources/StandardMacros.FlipFlop`
      (:`A`
        (set `self.Letter` true)
        (set `self.EndLetter` false))
      (:`B`
        (set `self.Letter` false)
        (set `self.EndLetter` true))))
  (`self.SpawnSegment` (`KismetMathLibrary.MakeTransform` (+ `Spawn Transform Location` (* (1610.0 0.0 0.0) (`self.DrawDistance`)))) (`KismetMathLibrary.RandomIntegerInRange` 1 5) (`KismetMathLibrary.RandomBool`) `DeleteOld?` (`self.Letter`) (`self.EndLetter`))
  (`/Engine/EditorBlueprintResources/StandardMacros.IncrementFloat` (`self.Counter`)
    (:`  `
      (set `self.Letter` false)
      (set `self.EndLetter` false))))

(fn `DeleteSegment`
  (bind _todelete (`self.ToDelete`)
    (:`then`
      (`self.K2_DestroyActor` _todelete))
    (:`else`)))

(fn `IncreaseEachNSeg`
  (params (Value :type "Float (double-precision)"))
  (set `self.EachNSegments` (+ (`self.EachNSegments`) Value)))

(fn `SpawnSegment`
  (params (SpawnTransform :type "Transform Structure") (`Num Lines` :type Integer) (`Prefer Left?` :type Boolean) (`DeleteOld?` :type Boolean) (`Letter?` :type Boolean) (`EndLetter?` :type Boolean))
  (bind _segments (`self.Segments`))
  (bind _output (`|GetArrayItem` _segments))
  (if `DeleteOld?`
    (`self.DeleteSegment`)
    (if (`KismetSystemLibrary.IsValid` _output)
      (set `self.ToDelete` _output)
      (`KismetArrayLibrary.Array_RemoveItem` _segments _output)))
  (bind _returnvalue (`|SpawnActorFromClass` "/Game/Blueprints/BP_RoadSegment.BP_RoadSegment_C" (`local.SpawnTransform`) "Undefined" "OverrideRootScale" null self `Num Lines` `Prefer Left?` `Letter?` `EndLetter?` null))
  (`KismetArrayLibrary.Array_Add` (`self.Segments`) _returnvalue))

(fn `UserConstructionScript`)