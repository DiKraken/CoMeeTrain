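; Road segment actor that builds a stretch of parallel lanes from spawned BP_Line actors and drives road progression as the player passes through.
; On BeginPlay it alternates lines either side of its origin, favoring left or right, and widens its borders to match.
; One-shot triggers pass borders to BP_Player on entry and signal the Manager to spawn the next segment on exit.
; Attached lines are destroyed with the segment.
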(event `self.ReceiveBeginPlay`
  ;[1 1 1] BeginPlay
  (`KismetArrayLibrary.Array_Clear` (`self.Lines`))
  (`self.FillSegment` (`self.Num Lines`) (`self.Prefer Left?`)))

(event `FillSegment`
  (params (NumLines :type Integer) (`PreferLeft?` :type Boolean))
  (bind _returnvalue (`self.K2_GetActorLocation`))
  (bind (_offset_x _offset_y) (`KismetMathLibrary.BreakVector` (`self.Offset`)))
  (bind _prefer_left_ (`self.Prefer Left?`))
  (bind _returnvalue_2 (`KismetMathLibrary.Abs` _offset_y))
  ;[1 1 1] FillAlghoritm
  (if (> NumLines 0)
    (if `PreferLeft?`
      (set `self.Offset` (`KismetMathLibrary.NegateVector` (`self.Offset`))))
    (`self.SpawnLine` (`KismetMathLibrary.MakeTransform` (`self.K2_GetActorLocation`)))
    (if (> (`self.Num Lines`) 1)
      (for _index (range 1 (`self.Num Lines`))
        (`/Engine/EditorBlueprintResources/StandardMacros.FlipFlop`
          (:`A`
            (`self.SpawnLine` (`KismetMathLibrary.MakeTransform` (+ (* (`self.Offset`) (- _index (`self.Minus`))) _returnvalue)))
            (`/Engine/EditorBlueprintResources/StandardMacros.IncrementInt` (`self.Minus`)
              (:`  `
                (if _prefer_left_
                  (set `self.Border Left` (- (`self.Border Left`) _returnvalue_2) :!label _label)
                  (else
                    (set `self.Border Right` (+ (`self.Border Right`) _returnvalue_2) :!label _label_2))))))
          (:`B`
            (`self.SpawnLine` (`KismetMathLibrary.MakeTransform` (+ _returnvalue (* (`KismetMathLibrary.NegateVector` (`self.Offset`)) (- _index (`self.Minus`))))))
            (if _prefer_left_
              (goto _label_2)
              (else
                (goto _label)))))))))

(event `self.BoxExit.OnComponentBeginOverlap`
  (params (OverlappedComponent :type "PrimitiveComponent Object Reference") (OtherActor :type "Actor Object Reference") (OtherComp :type "PrimitiveComponent Object Reference") (OtherBodyIndex :type Integer) (bFromSweep :type Boolean) (SweepResult :type "HitResult Structure (by ref)"))
  ;[1 1 1] OnPlayerExit
  (cast `/Game/Base/BP_Player` OtherActor)
  (`/Engine/EditorBlueprintResources/StandardMacros.DoOnce` false
    (:`Completed`
      (`/Game/Blueprints/BP_LinesManager.SpawnSegmentSignal` (`self.Manager`) (`self.K2_GetActorLocation`) true))))

(event `self.BoxEnter.OnComponentBeginOverlap`
  (params (OverlappedComponent :type "PrimitiveComponent Object Reference") (OtherActor :type "Actor Object Reference") (OtherComp :type "PrimitiveComponent Object Reference") (OtherBodyIndex :type Integer) (bFromSweep :type Boolean) (SweepResult :type "HitResult Structure (by ref)"))
  (bind _border_left (`self.Border Left`))
  (bind _border_right (`self.Border Right`))
  ;[1 1 1] OnPlayerEnter
  (bind _asbp_player (cast `/Game/Base/BP_Player` OtherActor))
  (`/Engine/EditorBlueprintResources/StandardMacros.DoOnce` false
    (:`Completed`
      (`/Game/Base/BP_Player.CheckUnder` _asbp_player)
      (`/Game/Base/BP_Player.SetBorders` _asbp_player _border_left _border_right)
      (`KismetSystemLibrary.PrintString` (`KismetStringLibrary.Concat_StrStr` (`KismetStringLibrary.Conv_DoubleToString` (/ _border_left 150.0)) " / " (`KismetStringLibrary.Conv_DoubleToString` (/ _border_right 150.0)))))))

(event `self.ReceiveDestroyed`
  ;[1 1 1] Destructor
  (for _array_element (`self.Lines`)
    (`self.K2_DestroyActor` _array_element)))

(fn `SpawnLine`
  (params (SpawnTransform :type "Transform Structure"))
  (bind _returnvalue (`|SpawnActorFromClass` "/Game/Blueprints/BP_Line.BP_Line_C" SpawnTransform "AlwaysSpawn" "OverrideRootScale" null null))
  (`self.K2_AttachToActor` _returnvalue self "None" "KeepWorld" "KeepWorld" "KeepWorld" true)
  (`KismetArrayLibrary.Array_Add` (`self.Lines`) _returnvalue))

(fn `UserConstructionScript`)